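; GrabMouse is the mouse drag-and-drop controller for a Tower of Hanoi-style puzzle with three tagged Towers and Rueda discs.
; A click line-traces from the cursor to grab an interactable Rueda.
; Tick snaps it above one of the towers based on cursor screen X.
; Release asks that Tower to validate the move, then places or returns the disc and shows the win screen when a non-start tower holds four.
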(event `Key|LeftMouseButton`
  (params (Key :type "Key Structure"))
  (bind _returnvalue (`GameplayStatics.GetPlayerController` 0))
  (bind _grabmode (`self.GrabMode`))
  (bind _grabcomponent (`self.GrabComponent`))
  (bind _ruedaactual (`self.RuedaActual`))
  (bind (_worldlocation _worlddirection) (`PlayerController.DeprojectMousePositionToWorld` (`GameplayStatics.GetPlayerController` 0)))
  (bind (_returnvalue_x _returnvalue_y) (`KismetMathLibrary.BreakVector` (`SceneComponent.K2_GetComponentLocation` _grabcomponent)))
  (bind _output (`|GetArrayItem` (`self.Towers`) (`self.TorreActual`)))
  (:`Pressed`
    (if _grabmode
      (bind (_outhit _returnvalue_2) (`KismetSystemLibrary.LineTraceSingle` _worldlocation (+ _worldlocation (* _worlddirection 10000.0)) "TraceTypeQuery1" true))
      (if _returnvalue_2
        (bind (_bblockinghit _binitialoverlap _time _distance _location _impactpoint _normal _impactnormal _physmat _hitactor _hitcomponent) (`GameplayStatics.BreakHitResult` _outhit))
        (if (== (`SceneComponent.Mobility` _hitcomponent) (enumliteral `EComponentMobility` "Movable"))
          (set `self.OriginalDistanceToObject` _distance)
          (bind _asrueda (cast `/Game/Blueprints/Rueda` (`ActorComponent.GetOwner` _hitcomponent)))
          (if (`/Game/Blueprints/Rueda.Interactable` _asrueda)
            (set `self.RuedaActual` _asrueda)
            (bind _output_get (set `self.GrabComponent` _hitcomponent))
            (set `self.OriginalPosition` (`SceneComponent.K2_GetComponentLocation` _output_get))
            (`GameplayStatics.PlaySoundAtLocation` "/Game/Music/131658__bertrof__game-sound-selection.131658__bertrof__game-sound-selection" (0.0 0.0 0.0) (struct) 1.0 1.0 0.0 null null null)
            (if (`SceneComponent.IsSimulatingPhysics` _output_get "None")
              (bind (_bblockinghit_2 _binitialoverlap_2 _time_2 _distance_2 _location_2 _impactpoint_2 _normal_2 _impactnormal_2 _physmat_2 _hitactor_2 _hitcomponent_2) (`GameplayStatics.BreakHitResult` _outhit))
              (`PhysicsHandleComponent.GrabComponentAtLocation` (`self.PhysicsHandle`) (`self.GrabComponent`) "None" _location_2)
              (else
                (set `self.RelativaGrabLocation` (`KismetMathLibrary.InverseTransformLocation` (`KismetMathLibrary.Conv_VectorToTransform` (`SceneComponent.K2_GetComponentLocation` _hitcomponent_2)) _location_2)))))))))
  (:`Released`
    (if _grabmode
      (`/Engine/EditorBlueprintResources/StandardMacros.IsValid` _ruedaactual
        (:`Is Valid`
          (bind (_valido _pos_z) (`/Game/Blueprints/Tower.CheckRueda` (`|GetArrayItem` (`self.Towers`) (`self.TorreActual`)) _ruedaactual))
          (if (not _valido)
            (`/Engine/EditorBlueprintResources/StandardMacros.IsValid` (`self.GrabComponent`)
              (:`Is Valid`
                (`SceneComponent.K2_SetWorldLocation` _grabcomponent (`self.OriginalPosition`) false true)
                (`GameplayStatics.PlaySoundAtLocation` "/Game/Music/476177__unadamlar__wrong-choice.476177__unadamlar__wrong-choice" (0.0 0.0 0.0) (struct) 1.0 1.0 0.0 null null null)))
            (else
              (`/Game/Blueprints/Tower.RemoveRueda` (`/Game/Blueprints/Rueda.ActualTower` (`self.RuedaActual`)))
              (`SceneComponent.K2_SetWorldLocation` _grabcomponent (`KismetMathLibrary.MakeVector` _returnvalue_x _returnvalue_y _pos_z) false true)
              (set `/Game/Blueprints/Rueda.ActualTower` _output (`self.RuedaActual`))))
          (set `self.GrabComponent` null)
          (`PhysicsHandleComponent.ReleaseComponent` (`self.PhysicsHandle`))
          (`GameplayStatics.PlaySoundAtLocation` "/Game/Music/218461__thomasjaunism__wood-block.218461__thomasjaunism__wood-block" (0.0 0.0 0.0) (struct) 1.0 1.0 0.0 null null null)
          (if (and (== (`/Game/Blueprints/Tower.CantidadRuedas` _output) 4) (not (`/Game/Blueprints/Tower.StartTower` _output)))
            (`/Game/Blueprints/Tower.FinishGame` _output)
            (`GameplayStatics.PlaySoundAtLocation` "/Game/Music/320672__rhodesmas__win-01.320672__rhodesmas__win-01" (0.0 0.0 0.0) (struct) 1.0 1.0 0.0 null null null)
            (bind _returnvalue_3 (`|CreateWidget` "/Game/Blueprints/WinScreen.WinScreen_C" _returnvalue))
            (`UserWidget.AddToViewport` _returnvalue_3 0)
            (set `PlayerController.bShowMouseCursor` true _returnvalue)))))))

(event `self.ReceiveBeginPlay`
  (bind _returnvalue (`GameplayStatics.GetPlayerController` 0))
  (for _index (range 1 4)
    (bind _outactors (`GameplayStatics.GetAllActorsWithTag` (`KismetStringLibrary.Conv_StringToName` (`KismetStringLibrary.Concat_StrStr` "Tower" (`KismetStringLibrary.Conv_IntToString` _index)))))
    (`KismetArrayLibrary.Array_Add` (`self.Towers`) (cast `/Game/Blueprints/Tower` (`|GetArrayItem` _outactors) :!pure true))
    (set `self.GrabMode` (not (`self.GrabMode`)))
    (set `PlayerController.bShowMouseCursor` (not (`PlayerController.bShowMouseCursor` _returnvalue)) _returnvalue)))

(event `self.ReceiveTick`
  (params (DeltaSeconds :type "Float (single-precision)"))
  (bind _grabcomponent (`self.GrabComponent`))
  (bind _locationx (`PlayerController.GetMousePosition` (`GameplayStatics.GetPlayerController` 0)))
  (bind _sizex (`PlayerController.GetViewportSize` (`GameplayStatics.GetPlayerController` 0)))
  (bind _returnvalue (* _sizex 0.6))
  (if (`self.GrabMode`)
    (`/Engine/EditorBlueprintResources/StandardMacros.IsValid` _grabcomponent
      (:`Is Valid`
        (if (`ActorComponent.ComponentHasTag` _grabcomponent "Rueda")
          (if (< _locationx (* _sizex 0.4))
            (`SceneComponent.K2_SetWorldLocation` _grabcomponent (330.0 -270.0 220.0) false false)
            (set `self.TorreActual` 0)
            (elif (< _locationx _returnvalue)
              (`SceneComponent.K2_SetWorldLocation` (`self.GrabComponent`) (330.0 -30.0 220.0) false false)
              (set `self.TorreActual` 1)
              (elif (> _locationx _returnvalue)
                (`SceneComponent.K2_SetWorldLocation` (`self.GrabComponent`) (340.0 240.0 220.0) false false)
                (set `self.TorreActual` 2)))))))))

(fn `UserConstructionScript`)