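; Tower Blueprint for a Tower of Hanoi-style puzzle peg that holds a stack of discs (Ruedas).
; CheckRueda accepts only a disc smaller than the current top, locks those beneath and returns a height from its stack index.
; RemoveRueda pops the top disc, then either re-enables the one below and restores its size limit or resets the limit when empty.
; FinishGame disables interaction on every stacked disc.
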(event `self.ReceiveTick`
  (params (DeltaSeconds :type "Float (single-precision)")))

(fn `CheckRueda`
  (params (Rueda :type "/Game/Blueprints/Rueda Object Reference"))
  (returns (Valido :type Boolean) (`Pos Z` :type "Float (double-precision)"))
  (bind _valor (`/Game/Blueprints/Rueda.Valor` Rueda))
  (bind _ruedareferencia (`self.RuedaReferencia`))
  (if (< _valor (`self.MaxRueda`))
    (set `self.MaxRueda` _valor)
    (bind _returnvalue (`KismetArrayLibrary.Array_Add` _ruedareferencia Rueda))
    (for (_array_element _array_index) _ruedareferencia
      (if (< _array_index (- (`KismetArrayLibrary.Array_Length` _ruedareferencia) 1))
        (set `/Game/Blueprints/Rueda.Interactable` false _array_element)))
    (set `self.CantidadRuedas` (+ _returnvalue 1))
    (return true (`KismetMathLibrary.Conv_IntToDouble` (+ (* _returnvalue 20) 50)))
    (else
      (return false 0.0))))

(fn `FinishGame`
  (for _array_element (`self.RuedaReferencia`)
    (set `/Game/Blueprints/Rueda.Interactable` false _array_element)))

(fn `RemoveRueda`
  (bind _cantidadruedas (`self.CantidadRuedas`))
  (`KismetArrayLibrary.Array_Remove` (`self.RuedaReferencia`) (- _cantidadruedas 1))
  (bind _result (`/Engine/EditorBlueprintResources/StandardMacros.DecrementInt` _cantidadruedas)
    (:`  `
      (if (== _result 0)
        (set `self.MaxRueda` 5)
        (else
          (bind _output (`|GetArrayItem` (`self.RuedaReferencia`) (- _result 1)))
          (set `/Game/Blueprints/Rueda.Interactable` true _output)
          (set `self.MaxRueda` (`/Game/Blueprints/Rueda.Valor` _output)))))))

(fn `UserConstructionScript`)